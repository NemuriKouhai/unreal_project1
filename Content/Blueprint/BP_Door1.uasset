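; BP_Door1 is a door that swings open when a BPTest actor enters its Box trigger, either freely or by consuming a key.
; A DoorName of "None" opens it directly; otherwise the game instance must report that key as Got, then saves it as Used.
; A timeline animates Door1's yaw.
; On completion, the SetEventFinished override calls its parent, snaps the door to 90 degrees and disables the trigger's collision.
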(event `self.Box.OnComponentBeginOverlap`
  (params (OverlappedComponent :type "PrimitiveComponent Object Reference") (OtherActor :type "Actor Object Reference") (OtherComp :type "PrimitiveComponent Object Reference") (OtherBodyIndex :type Integer) (bFromSweep :type Boolean) (SweepResult :type "HitResult Structure (by ref)"))
  (cast `/Game/Blueprint/BPTest` OtherActor)
  (if (== (`self.DoorName`) "None")
    (`self.OpenDoor`)
    (else
      (switch `/Game/Blueprint/KeyStatus` (`/Game/Blueprint/BP_MyGameInstance.GetKeyStatus` (`self.MyGameInstance`) (`self.DoorName`))
        (:`NewEnumerator1`
          (`/Game/Blueprint/BP_MyGameInstance.SaveKeyStatus` (`self.MyGameInstance`) (`self.DoorName`) "NewEnumerator2")
          (`self.OpenDoor`))))))

(event `OpenDoor`
  (set `self.switchdoor` false)
  (bind (_direction _openz) (`Timeline|タイムライン_0`)
    (:`Update`
      (`SceneComponent.K2_SetRelativeRotation` (`self.door1`) (`KismetMathLibrary.MakeRotator` 0.0 0.0 _openz) false false))
    (:`Finished`
      (`self.SetEventFinished`))))

(event `self.ReceiveBeginPlay`
  (`parent.ReceiveBeginPlay`))

(fn `SetEventFinished`
  (`parent.SetEventFinished`)
  (`SceneComponent.K2_SetRelativeRotation` (`self.door1`) (struct :`Yaw` 90.0) false false)
  (`PrimitiveComponent.SetCollisionEnabled` (`self.Box`) "NoCollision")
  (set `self.switchdoor` false))

(fn `UserConstructionScript`)