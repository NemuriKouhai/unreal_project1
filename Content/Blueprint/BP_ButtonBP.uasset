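; Floor button that opens a linked door when the player steps into its trigger box.
; The overlap plays the Pushed timeline, which animates the button's height, then, if DoorToOpen is valid, marks the event finished and enables that door.
; The SetEventFinished override calls the parent, snaps the button to its lowered position and disables the box's collision.
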(event `self.ReceiveBeginPlay`
  (`parent.ReceiveBeginPlay`))

(event `self.Box.OnComponentBeginOverlap`
  (params (OverlappedComponent :type "PrimitiveComponent Object Reference") (OtherActor :type "Actor Object Reference") (OtherComp :type "PrimitiveComponent Object Reference") (OtherBodyIndex :type Integer) (bFromSweep :type Boolean) (SweepResult :type "HitResult Structure (by ref)"))
  (cast `/Game/Blueprint/BP_Player` OtherActor)
  (bind (_direction `_新規track_0`) (`Timeline|pushed`)
    (:`Update`
      (`SceneComponent.K2_SetRelativeLocation` (`self.buttonPushed`) (`KismetMathLibrary.MakeVector` 0.0 0.0 `_新規track_0`) false false))
    (:`Finished`
      (bind _doortoopen (`self.DoorToOpen`)
        (:`then`
          (`self.SetEventFinished`)
          (`/Game/Blueprint/BP_MovingBox.enable` _doortoopen))
        (:`else`)))))

(fn `SetEventFinished`
  (`parent.SetEventFinished`)
  (`SceneComponent.K2_SetRelativeLocation` (`self.buttonPushed`) (0.0 0.0 -25.0) false false)
  (`PrimitiveComponent.SetCollisionEnabled` (`self.Box`) "NoCollision"))

(fn `UserConstructionScript`)